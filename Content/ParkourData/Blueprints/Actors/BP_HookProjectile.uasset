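; BP_HookProjectile is the grappling hook projectile actor for the parkour system.
; On begin play it records its starting position and sets its collision sphere to ignore the instigator while moving.
; Each tick it checks the distance travelled and destroys itself beyond MaxRange.
; When the sphere hits something, it sends the impact location to the owner's ParkourComponent through GrapplingHookHitMessage.
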(event OnComponentHit(Sphere)
  (params (HitComponent :type Primitive%20Component%20Object%20Reference) (OtherActor :type Actor%20Object%20Reference) (OtherComp :type Primitive%20Component%20Object%20Reference) (NormalImpulse :type Vector :default "0, 0, 0") (Hit :type Hit%20Result%20Structure%20%28by%20ref%29))
  (Class|CombatBPI|GrapplingHookHit(Message) (Actor|GetComponentbyClass (Components|GetOwner) "/Game/ParkourData/Blueprints/Components/ParkourComponent.ParkourComponent_C") (.location Hit)))

(event EventBeginPlay
  (Collision|IgnoreActorwhenMoving (Variables|Default|GetSphere) (Game|GetInstigator) true)
  (bind _output_get (Variables|Default|SetStaringPostion (Transformation|GetActorLocation))))

(event EventTick
  (params (DeltaSeconds :type Float%20%28single-precision%29))
  (if (> (Math|Vector|Distance(Vector) (stale EventBeginPlay _output_get) (Transformation|GetActorLocation)) (Variables|Default|GetMaxRange))
    (Utilities|FlowControl|DoOnce false
      (:Completed
        (Actor|DestroyActor)))))

(fn ConstructionScript)