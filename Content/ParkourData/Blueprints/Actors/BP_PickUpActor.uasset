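; BP_PickUpActor is a world pickup that hands an item to whoever interacts with it.
; Interact spawns the configured Item class at the pickup's transform with the caller as owner and instigator, calls OnEquipped on it, then destroys the pickup.
; PulltoPlayer tosses the physics Cube toward a given actor with a velocity-change impulse plus an upward lift.
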(event EventPulltoPlayer
  (params (Actor :type Vector :default "0, 0, 0"))
  (Physics|AddImpulse (Variables|Default|GetCube) (+ (* (Math|Vector|GetForwardVector (Math|Rotator|FindLookatRotation (Transformation|GetWorldLocation (Variables|Default|GetCube)) Actor)) 8.0) "0.000000,0.000000,8.000000") "None" true))

(event EventInteract
  (params (CallEvent :type Actor%20Object%20Reference))
  (bind _returnvalue (Game|SpawnActorfromClass (Variables|Default|GetItem) (Transformation|GetActorTransform) "Undefined" "MultiplyWithRoot" CallEvent (.AsPawn (Utilities|Casting|CastToPawn CallEvent))))
  (Default|OnEquipped _returnvalue)
  (Actor|DestroyActor))

(fn ConstructionScript)