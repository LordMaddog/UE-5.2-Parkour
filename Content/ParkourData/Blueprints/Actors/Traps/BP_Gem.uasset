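; BP_Gem is a trap that fires bursts of five BP_IceT1 projectiles at any Character entering its Activater volume.
; Overlap begin stores the target and fires immediately, while Tick gated by a ReFireTime Delay repeats bursts until overlap ends.
; Each shot spawns at FireSpot, re-aimed at the target's current location, with damage, range, speed and impact explosion passed through.
; The construction script sets trigger visibility and offset, and scales Scene.
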(event OnComponentBeginOverlap(Activater)
  (params (OverlappedComponent :type Primitive%20Component%20Object%20Reference) (OtherActor :type Actor%20Object%20Reference) (OtherComp :type Primitive%20Component%20Object%20Reference) (OtherBodyIndex :type Integer) (bFromSweep :type Boolean) (SweepResult :type Hit%20Result%20Structure%20%28by%20ref%29))
  (bind _spawn_transform_scale (Variables|Projectile|GetSpawn%20Transform%20Scale))
  (bind _firespot (Variables|Default|GetFireSpot))
  (bind _returnvalue (Transformation|GetWorldLocation _firespot))
  (bind _ascharacter (Utilities|Casting|CastToCharacter OtherActor))
  (Variables|Default|SetCharacter _ascharacter)
  (Variables|Projectile|SetStill%20Over%20Laping true)
  (Variables|Default|SetShotsFired 0.0)
  (Game|SpawnActorfromClass "/Game/ParkourData/Blueprints/Actors/Magic/BP_IceT1.BP_IceT1_C" (Math|Transform|MakeTransform _returnvalue (Math|Rotator|FindLookatRotation _returnvalue (Transformation|GetActorLocation (Variables|Default|GetCharacter))) (Math|Vector|MakeVector _spawn_transform_scale _spawn_transform_scale _spawn_transform_scale)) "Undefined" "MultiplyWithRoot" self (Variables|Projectile|GetMax%20Range) 1e+02 (Variables|Projectile|GetBase%20Damage) (Variables|Projectile|GetInitial%20Speed) (Variables|Projectile|GetExplod%20on%20Impact) 0 :!label _label)
  (Math|Float|IncrementFloat (Variables|Default|GetShotsFired)
    (:%20%20
      (Utilities|FlowControl|Delay 0.1)
      (if (< (Variables|Default|GetShotsFired) 5.0)
        (goto _label)))))

(event OnComponentEndOverlap(Activater)
  (params (OverlappedComponent :type Primitive%20Component%20Object%20Reference) (OtherActor :type Actor%20Object%20Reference) (OtherComp :type Primitive%20Component%20Object%20Reference) (OtherBodyIndex :type Integer))
  (Utilities|Casting|CastToCharacter OtherActor)
  (Variables|Projectile|SetStill%20Over%20Laping false))

(event EventTick
  (params (DeltaSeconds :type Float%20%28single-precision%29))
  (bind _spawn_transform_scale (Variables|Projectile|GetSpawn%20Transform%20Scale))
  (bind _firespot (Variables|Default|GetFireSpot))
  (bind _returnvalue (Transformation|GetWorldLocation _firespot))
  (Utilities|FlowControl|Delay (Variables|Projectile|GetReFireTime))
  (if (Variables|Projectile|GetStill%20Over%20Laping)
    (Utilities|IsValid (Variables|Default|GetCharacter)
      (:Is%20Valid
        (Variables|Default|SetShotsFired 0.0)
        (Game|SpawnActorfromClass "/Game/ParkourData/Blueprints/Actors/Magic/BP_IceT1.BP_IceT1_C" (Math|Transform|MakeTransform _returnvalue (Math|Rotator|FindLookatRotation _returnvalue (Transformation|GetActorLocation (Variables|Default|GetCharacter))) (Math|Vector|MakeVector _spawn_transform_scale _spawn_transform_scale _spawn_transform_scale)) "Undefined" "MultiplyWithRoot" self (Variables|Projectile|GetMax%20Range) 1e+02 (Variables|Projectile|GetBase%20Damage) (Variables|Projectile|GetInitial%20Speed) (Variables|Projectile|GetExplod%20on%20Impact) 0 :!label _label)
        (Math|Float|IncrementFloat (Variables|Default|GetShotsFired)
          (:%20%20
            (Utilities|FlowControl|Delay 0.1)
            (if (< (Variables|Default|GetShotsFired) 5.0)
              (goto _label))))))))

(fn ConstructionScript
  (Rendering|SetVisibility (Variables|Default|GetActivater) (Variables|ActiveArea|GetColiderVisible) false)
  (Transformation|SetWorldScale3D (Variables|Default|GetScene) (Variables|ActiveArea|GetIn%20Box%20Extent))
  (Transformation|SetRelativeLocation (Variables|Default|GetActivater) (Math|Vector|MakeVector 0.0 (Variables|ActiveArea|GetOfset) 0.0) false false))