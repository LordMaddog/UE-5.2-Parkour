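; BP_BaseWeapon is the base weapon actor that attaches to a character, registers with its combat component and supplies montages per action type.
; Melee weapons toggle collision, trail and swing sound, applying point damage on hit, while magic weapons attach hand sparks and message the combat component.
; Timelines float the weapon out beside the owner with idle bobbing, then return it to hand.
; It also drives fire enchant effects and drops via physics.
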(event OnHit(CollosionComponent)
  (params (HitResult :type Hit%20Result%20Structure))
  (bind (_bblockinghit _binitialoverlap _time _distance _location _impactpoint _normal _impactnormal _physmat _hitactor _hitcomponent) (Collision|BreakHitResult HitResult))
  (bind _returnvalue (Class|CombatBPI|CanReciveDamage(Message) _hitactor))
  (if _returnvalue
    (Game|Damage|ApplyPointDamage _hitactor (Variables|Default|GetBase%20Damage) (Transformation|GetActorForwardVector (Components|GetOwner)) HitResult (Game|GetInstigatorController) self)))

(event Custom|ActivateDamage
  (params (LeftHand :type Boolean))
  ;[1 1 1] Activate/Deactivate Weapon
  (if (not (Variables|Default|GetIsMagic))
    (CallFunction|MeleeActivate)
    (else
      (Class|CombatBPI|MagicSpawn(Message) (Variables|Default|GetCombatComponent) true LeftHand))))

(event Custom|DeActivateDamage
  ;[1 1 1] Activate/Deactivate Weapon
  (if (not (Variables|Default|GetIsMagic))
    (Default|DisableCollision (Variables|Default|GetCollosionComponent))
    (Utilities|FlowControl|RetriggerableDelay 0.1)
    (Components|Activation|Deactivate (Variables|Default|GetN_WeaponTrail))
    (Effects|Components|ParticleSystem|SetBoolParameter (Variables|Default|GetN_FireEnchantment) "Trail" false)
    (else
      (Class|CombatBPI|MagicSpawn(Message) (Variables|Default|GetCombatComponent) false false))))

(event Custom|FireEnchant
  (params (Active :type Boolean))
  (bind _n_fireenchantment (Variables|Default|GetN_FireEnchantment))
  ;[1 1 1] MagicEnchantMents
  (bind _output_get (Variables|Magic|SetFireInchant%20active Active))
  (if _output_get
    (Components|Activation|Activate _n_fireenchantment false)
    (else
      (Components|Activation|Deactivate _n_fireenchantment))))

(event Custom|EnchantPowerSet
  (params (EnchantPowerSet :type Float%20%28double-precision%29))
  ;[1 1 1] Magic particel effect strangth
  (Effects|Components|ParticleSystem|SetFloatParameter (Variables|Default|GetN_FireEnchantment) "SpawnRate" EnchantPowerSet))

(event Custom|SimulatePhysics
  (bind _return_value (CallFunction|GetItemMesh))
  ;[1 1 1] Drop Weapon - hapens on death or disarm
  (Collision|SetCollisionProfileName _return_value "PhysicsActor" true :!class /Script/Engine.PrimitiveComponent)
  (Physics|SetSimulatePhysics _return_value true))

(event Custom|WeaponFloat
  (params (FloatAway :type Boolean))
  (bind _floatmagiceffect (Variables|Default|GetFloatMagicEffect))
  ;[1 1 1] WeaponFloat
  (if FloatAway
    (Components|Activation|Activate _floatmagiceffect true)
    (CallFunction|DeActivateDamage)
    (bind _floattime (Timeline|FloatAway PlayFromStart)
      (:Update
        (bind _returnvalue (Utilities|FloatAwayVector _floattime _floattime FloatAway)))
      (:Finished
        (Variables|Default|SetRandom%20Float%201 (Math|Random|RandomFloatinRange -1e+01 1e+01) :!label _label)
        (Variables|Default|SetRandom%20Float%202 (Math|Random|RandomFloatinRange -1e+01 1e+01))
        (bind _floattime_2 (Timeline|TimelineMagicIdleFloat PlayFromStart)
          (:Update
            (if FloatAway
              (Transformation|SetActorLocation (|Switch _floattime_2 _returnvalue) false false)
              (Utilities|FlowControl|RetriggerableDelay 0.01)
              (goto _label))))))
    (else
      (Components|Activation|Deactivate _floatmagiceffect)
      (bind _floattime_3 (Timeline|Timeline PlayFromStart)
        (:Update
          (Utilities|FloatBackVector _floattime_3 _floattime_3 false))))))

(event EventBeginPlay
  ;[1 1 1] Defualt
  (|CallParentFunction)
  (CallFunction|MagicHands))

(event Collision|EventActorBeginOverlap
  (params (OtherActor :type Actor%20Object%20Reference))
  ;[1 1 1] Defualt
  (|CallParentFunction OtherActor) ; This node is disabled and will not be called.\nDrag off pins to build functionality.
)

(event EventTick
  (params (DeltaSeconds :type Float%20%28single-precision%29))
  ;[1 1 1] Defualt
  (|CallParentFunction DeltaSeconds) ; This node is disabled and will not be called.\nDrag off pins to build functionality.
)

(fn ConstructionScript
  (bind _sword_langth (Variables|Initialization|GetSword%20Langth))
  (|CallParentFunction)
  (Effects|Components|ParticleSystem|SetFloatParameter (Variables|Default|GetN_WeaponTrail) "Ribbon Width" _sword_langth)
  (Effects|Components|ParticleSystem|SetFloatParameter (Variables|Default|GetN_FireEnchantment) "SwordHight" (* _sword_langth 2.0))
  (Effects|Components|ParticleSystem|SetFloatParameter (Variables|Default|GetN_FireEnchantment) "SpawnRate" (Variables|Magic|GetEnchantmentPower))
  (Effects|Components|ParticleSystem|SetBoolParameter (Variables|Default|GetN_FireEnchantment) "Trail" false))

(fn OnEquipped
  (Variables|Default|SetCombatComponent (Actor|GetComponentbyClass (Components|GetOwner) "/Game/ParkourData/Blueprints/Components/ParkourComponent.ParkourComponent_C"))
  (CallFunction|SetEquipped true)
  (CallFunction|AttachActor (select (Default|GetCombatEnabled (Variables|Default|GetCombatComponent)) (Variables|Initialization|GetHandSocketName) (Variables|Default|GetAttachSocket%20Name)) "SnapToTarget")
  (Default|SetMainWeapon (Variables|Default|GetCombatComponent) self)
  (Class|AnimBPI|CombatType(Message) (Components|SkeletalMesh|GetAnimInstance (Variables|/Script/Engine.Character|GetMesh (.AsCharacter (Utilities|Casting|CastToCharacter (Components|GetOwner))))) (Variables|Initialization|GetCombatTypes))
  (Default|SetCollisionMesh (Variables|Default|GetCollosionComponent) (CallFunction|GetItemMesh))
  (Default|AddActortoIgnore (Variables|Default|GetCollosionComponent) (Components|GetOwner)))

(fn GetActionMontages
  (params (Index :type E_CharacterActions%20Enum :default "NewEnumerator0"))
  (return (Utilities|Select :Index Index :NewEnumerator0 0 :NewEnumerator7 0 :NewEnumerator11 (Variables|Animations|GetSprintAttackMontages) :NewEnumerator1 (Variables|Animations|GetLightAttackMontages) :NewEnumerator2 (Variables|Animations|GetHeavyAttackMontages) :NewEnumerator9 (Variables|Animations|GetChargeAttackMontages) :NewEnumerator10 (Variables|Animations|GetAirAttackMontages) :NewEnumerator3 (Variables|Animations|GetPlungAttackMontages) :NewEnumerator4 (Variables|Animations|GetDodgeMontages) :NewEnumerator5 (Utilities|Array|MakeArray (Variables|Animations|GetEnterCombat)) :NewEnumerator6 (Utilities|Array|MakeArray (Variables|Animations|GetExitCombat)) :NewEnumerator8 0)))

(fn MeleeActivate
  (Default|EnableCollision (Variables|Default|GetCollosionComponent))
  (Components|Activation|Activate (Variables|Default|GetN_WeaponTrail) false)
  (Effects|Components|ParticleSystem|SetBoolParameter (Variables|Default|GetN_FireEnchantment) "Trail" true)
  (Components|Activation|Activate (Variables|Default|GetSwingSound) true))

(fn MagicHands
  (if (Variables|Default|GetIsMagic)
    (Transformation|AttachComponentToComponent (Variables|Default|GetRightHandMagicSparks) (Variables|/Script/Engine.Character|GetMesh (.AsCharacter (Utilities|Casting|CastToCharacter (Components|GetOwner)))) (Variables|Initialization|GetHandRightSocketName) "SnapToTarget" "SnapToTarget" "SnapToTarget" true)
    (Transformation|AttachComponentToComponent (Variables|Default|GetLeftHandMagicSparks) (Variables|/Script/Engine.Character|GetMesh (.AsCharacter (Utilities|Casting|CastToCharacter (Components|GetOwner)))) (Variables|Initialization|GetHandLeftSocketName) "SnapToTarget" "SnapToTarget" "SnapToTarget" true)
    (Components|Activation|Activate (Variables|Default|GetLeftHandMagicSparks) false)
    (Variables|Default|SetCombatComponent (Actor|GetComponentbyClass (Components|GetOwner) "/Game/ParkourData/Blueprints/Components/ParkourComponent.ParkourComponent_C"))))