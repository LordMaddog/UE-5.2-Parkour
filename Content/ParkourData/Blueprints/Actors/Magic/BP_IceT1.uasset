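; Tier-one ice spike magic projectile that ignores its instigator and destroys itself beyond a maximum range.
; On first hit it deals point damage, then either explodes or sticks.
; Stuck spikes attach to the character bone (ragdolling and pushing BP_PC) or become blockers on other actors, then shrink away via timeline.
; Explosions, also triggered by sufficient incoming damage, point-damage actors overlapping a construction-sized sphere, then destroy the projectile.
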(event OnComponentHit(MainProjectile)
  (params (HitComponent :type Primitive%20Component%20Object%20Reference) (OtherActor :type Actor%20Object%20Reference) (OtherComp :type Primitive%20Component%20Object%20Reference) (NormalImpulse :type Vector :default "0, 0, 0") (Hit :type Hit%20Result%20Structure%20%28by%20ref%29))
  (bind _returnvalue (* (.location Hit) 1e+01))
  (Variables|Default|SetOther%20Actor OtherActor)
  (Variables|Default|SetHit (Collision|MakeHitResult (.bblockinghit Hit) (.binitialoverlap Hit) (.time Hit) (.distance Hit) (.location Hit) (.impactpoint Hit) (.normal Hit) (.impactnormal Hit) (.physmat Hit) (.hitactor Hit) (.hitcomponent Hit) (.hitbonename Hit) (.bonename Hit) (.hititem Hit) (.elementindex Hit) (.faceindex Hit) (.tracestart Hit) (.traceend Hit)))
  (Utilities|FlowControl|DoOnce false
    (:Completed
      (Components|Activation|Activate (Variables|Default|GetP_Trap_Blast_Ice_01_Converted) true)
      (Audio|Components|Audio|Stop (Variables|Default|GetFlySound))
      (Game|Damage|ApplyPointDamage (Variables|Default|GetOther%20Actor) (Variables|Default|GetBase%20Damage) _returnvalue (Variables|Default|GetHit) (Game|GetInstigatorController) (Game|GetInstigator))
      (if (not (Variables|Default|GetExplodOnImpact))
        (bind _ascharacter (Utilities|Casting|CastToCharacter (Variables|Default|GetOther%20Actor))
          (:then
            (Transformation|AttachComponentToComponent (Variables|Default|GetMainProjectile) (Variables|/Script/Engine.Character|GetMesh _ascharacter) (.hitbonename Hit) "KeepWorld" "KeepWorld" "KeepWorld" true)
            (Collision|SetCollisionEnabled (Variables|Default|GetMainProjectile) "NoCollision")
            (bind _asbp_pc (Utilities|Casting|CastToBP_PC (Variables|Default|GetOther%20Actor))
              (:then
                (Default|EnableRagdoll (Variables|/Game/ParkourData/BP_PC.BP_PC_C|GetParkourComponent _asbp_pc)))
              (:CastFailed
                _))
            (Utilities|FlowControl|Delay 0.01)
            (Physics|AddImpulse (Variables|/Script/Engine.Character|GetMesh _asbp_pc) _returnvalue (.hitbonename Hit) false))
          (:CastFailed
            (Utilities|IsValid (Variables|Default|GetOther%20Actor)
              (:Is%20Valid
                (Transformation|AttachActorToActor (Variables|Default|GetOther%20Actor) (.hitbonename Hit) "KeepWorld" "KeepWorld" "KeepWorld" true)
                (Collision|SetCollisionObjectType (Variables|Default|GetIceSpike) "ECC_WorldStatic")
                (Collision|SetCollisionResponsetoChannel (Variables|Default|GetIceSpike) "ECC_Pawn" "ECR_Block")
                (Collision|SetCollisionEnabled (Variables|Default|GetIceSpike) "QueryAndPhysics")
                (Collision|SetCollisionEnabled (Variables|Default|GetMainProjectile) "NoCollision")
                (Utilities|FlowControl|Delay 0.1)))))
        (Variables|Default|SetSize (Transformation|GetWorldScale (Variables|Default|GetIceSpike)))
        (bind _newtrack_0 (Timeline|Shrink PlayFromStart)
          (:Update
            (Transformation|SetWorldScale3D (Variables|Default|GetIceSpike) (Math|Vector|Lerp(Vector) (Variables|Default|GetSize) "0, 0, 0" _newtrack_0)))
          (:Finished
            (Actor|DestroyActor)))
        (else
          (CallFunction|ExplodonImpact!))))))

(event Custom|ExplodOnImpact!
  (for _array_element (Collision|GetOverlappingActors (Variables|Default|GetSphere) 0 :!class /Script/Engine.PrimitiveComponent)
    (Game|Damage|ApplyPointDamage _array_element (Variables|Default|GetBase%20Damage) (Transformation|GetWorldLocation (Variables|Default|GetIceSpike)) (Variables|Default|GetHit) (Game|GetInstigatorController) (Game|GetInstigator)))
  (Components|Activation|Activate (Variables|Default|GetP_Buff) true)
  (Utilities|FlowControl|Delay 0.2)
  (Actor|DestroyActor))

(event EventBeginPlay
  (Collision|IgnoreActorwhenMoving (Variables|Default|GetMainProjectile) (Game|GetInstigator) true)
  (bind _output_get (Variables|Default|SetStaringPostion (Transformation|GetActorLocation))))

(event Game|Damage|EventAnyDamage
  (params (Damage :type Float%20%28single-precision%29) (DamageType :type Damage%20Type%20Object%20Reference) (InstigatedBy :type Controller%20Object%20Reference) (DamageCauser :type Actor%20Object%20Reference))
  (Variables|Default|SetDamageIn Damage)
  (if (>= (Variables|Default|GetDamageIn) 1e+01)
    (Utilities|FlowControl|DoOnce false
      (:Completed
        (for _array_element (Collision|GetOverlappingActors (Variables|Default|GetSphere) 0 :!class /Script/Engine.PrimitiveComponent)
          (Game|Damage|ApplyPointDamage _array_element (Variables|Default|GetBase%20Damage) (Transformation|GetWorldLocation (Variables|Default|GetIceSpike)) (Variables|Default|GetHit) (Game|GetInstigatorController) (Game|GetInstigator)))
        (Components|Activation|Activate (Variables|Default|GetP_Buff) true)
        (Utilities|FlowControl|Delay 0.2)
        (Actor|DestroyActor)))))

(event EventTick
  (params (DeltaSeconds :type Float%20%28single-precision%29))
  (if (> (Math|Vector|Distance(Vector) (stale EventBeginPlay _output_get) (Transformation|GetActorLocation)) (Variables|Default|GetMaxRange))
    (Utilities|FlowControl|DoOnce false
      (:Completed
        (Actor|DestroyActor)))))

(fn ConstructionScript
  (Components|Sphere|SetSphereRadius (Variables|Default|GetSphere) (Variables|Default|GetEplosive%20Radius) true)
  (Variables|/Script/Engine.ProjectileMovementComponent|SetInitialSpeed (Variables|Default|GetProjectileMovement) (Variables|Default|GetInitial%20Speed)))