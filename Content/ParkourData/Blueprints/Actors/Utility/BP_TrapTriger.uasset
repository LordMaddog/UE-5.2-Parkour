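; BP_TrapTriger is a trap trigger that makes a referenced BP_PC character fire a burst of magic when the player overlaps its capsule.
; The overlap resets a shot counter, then calls MagicCast on that character's ParkourComponent in a delayed loop until the counter passes its limit.
; The caster comes from the CharRef variable rather than the overlapping actor, and nothing blocks retriggering during a burst.
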(event OnComponentBeginOverlap(Capsule)
  (params (OverlappedComponent :type Primitive%20Component%20Object%20Reference) (OtherActor :type Actor%20Object%20Reference) (OtherComp :type Primitive%20Component%20Object%20Reference) (OtherBodyIndex :type Integer) (bFromSweep :type Boolean) (SweepResult :type Hit%20Result%20Structure%20%28by%20ref%29))
  (if (== OtherActor (Game|GetPlayerCharacter 0))
    (Variables|Default|SetFiredShots 0)
    (bind _asbp_combat_character (Utilities|Casting|CastToBP_PC (Variables|Default|GetCharRef)))
    (Default|MagicCast (Variables|/Game/ParkourData/BP_PC.BP_PC_C|GetParkourComponent _asbp_combat_character) "NewEnumerator1" :!label _label)
    (Utilities|FlowControl|Delay 0.5)
    (bind _result (Math|Integer|IncrementInt (Variables|Default|GetFiredShots))
      (:%20%20
        (if (<= _result 3)
          (goto _label))))))

(fn ConstructionScript)