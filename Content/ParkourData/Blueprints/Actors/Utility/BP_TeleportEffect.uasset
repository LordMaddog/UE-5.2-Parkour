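; BP_TeleportEffect is a short-lived actor that teleports and revives the player character (BP_PC) that overlaps its capsule.
; A one-shot overlap plays a get-up montage, disables movement, hides the meshes, then turns off collision after a delay.
; A timeline lerps the character to above TeleportLock, then moves the effect there, activates particles and audio, and restores movement, visibility, collision, a stat and parkour state before standing up.
; The actor destroys itself on a fixed timer from BeginPlay.
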(event OnComponentBeginOverlap(Capsule)
  (params (OverlappedComponent :type Primitive%20Component%20Object%20Reference) (OtherActor :type Actor%20Object%20Reference) (OtherComp :type Primitive%20Component%20Object%20Reference) (OtherBodyIndex :type Integer) (bFromSweep :type Boolean) (SweepResult :type Hit%20Result%20Structure%20%28by%20ref%29))
  (bind _asbp_pc (Utilities|Casting|CastToBP_PC OtherActor))
  (Variables|Default|SetCharacter _asbp_pc)
  (Utilities|FlowControl|DoOnce false
    (:Completed
      (Animation|PlayAnimMontage (Variables|Default|GetCharacter) "/Game/ParkourData/Animations/GetUp/Getting_UpFromFrontParticles_Montage.Getting_UpFromFrontParticles_Montage" 1.0 "None")
      (Pawn|Components|CharacterMovement|DisableMovement (Variables|/Script/Engine.Character|GetCharacterMovement (Variables|Default|GetCharacter)))
      (Development|SetHiddeninGame (Variables|/Script/Engine.Character|GetMesh (Variables|Default|GetCharacter)) true false)
      (Utilities|FlowControl|Delay 1.0)
      (Collision|SetActorEnableCollision (Variables|Default|GetCharacter) false)
      (Utilities|IsValid (Variables|Default|GetCharacter)
        (:Is%20Valid
          (Variables|Default|SetStart (Transformation|GetActorLocation (Variables|Default|GetCharacter)))
          (bind _duration (Timeline|TeleportTime PlayFromStart)
            (:Update
              (Transformation|SetActorLocation (Variables|Default|GetCharacter) (Math|Vector|Lerp(Vector) (Variables|Default|GetStart) (+ (Variables|Default|GetTeleport%20Lock) "0,0,200.000000") _duration) false true))
            (:Finished
              (Transformation|SetActorLocation (- (Transformation|GetWorldLocation (Variables|/Script/Engine.Character|GetMesh (Variables|Default|GetCharacter))) "0,0,15.000000") false true)
              (Components|Activation|Activate (Variables|Default|GetTeleportParticels) false)
              (Variables|/Script/Engine.Pawn|SetbUseControllerRotationPitch (Variables|Default|GetCharacter) false)
              (Transformation|SetActorRotation (Variables|Default|GetCharacter))
              (Pawn|Components|CharacterMovement|SetMovementMode (Variables|/Script/Engine.Character|GetCharacterMovement (Variables|Default|GetCharacter)) "MOVE_Walking" 0)
              (Development|SetHiddeninGame (Variables|/Script/Engine.Character|GetMesh (Variables|Default|GetCharacter)) false false)
              (Default|SetState (Variables|/Game/ParkourData/BP_PC.BP_PC_C|GetParkourComponent (Variables|Default|GetCharacter)) "NewEnumerator0")
              (Default|SetCurrentStatValue (Variables|/Game/ParkourData/BP_PC.BP_PC_C|GetStatsComponent (Variables|Default|GetCharacter)) "NewEnumerator1" 1e+02)
              (Collision|SetActorEnableCollision (Variables|Default|GetCharacter) true)
              (Variables|/Game/ParkourData/Blueprints/Components/ParkourComponent.ParkourComponent_C|SetbDead (Variables|/Game/ParkourData/BP_PC.BP_PC_C|GetParkourComponent (Variables|Default|GetCharacter)) false)
              (Default|StandUp (Variables|/Game/ParkourData/BP_PC.BP_PC_C|GetParkourComponent (Variables|Default|GetCharacter))))))))))

(event EventBeginPlay
  (Utilities|FlowControl|Delay 6.0)
  (Actor|DestroyActor))

(event EventTick
  (params (DeltaSeconds :type Float%20%28single-precision%29)))

(fn ConstructionScript)