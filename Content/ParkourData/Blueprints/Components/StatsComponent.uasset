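; Actor component that stores and manages character stats for the parkour game, including applying damage and death.
; Base stats map each stat to base and max values, and initialization copies base values into a current-value map.
; Modifications clamp current values between zero and the stat's max.
; TakeDamage lowers one stat and, at zero, calls Die on the owner's ParkourComponent, returning whether it died.
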(fn SetCurrentStatValue
  (params (Stat :type E_Stats%20Enum :default "NewEnumerator0") (Value :type Float%20%28double-precision%29))
  (Utilities|Map|Add (Variables|Stats|GetCurrentStats) Stat Value))

(fn GetCurrentStatValue
  (params (Stat :type E_Stats%20Enum :default "NewEnumerator0"))
  (return (.Value (Utilities|Map|Find (Variables|Stats|GetCurrentStats) Stat))))

(fn InitializeStats
  (bind _keys (Utilities|Map|Keys (Variables|BaseStats|GetBaseStats)))
  (for _array_element _keys
    (CallFunction|SetCurrentStatValue _array_element (.basevalue (.Value (Utilities|Map|Find (Variables|BaseStats|GetBaseStats) _array_element))))))

(fn ModifyCurrentStatValue
  (params (Stat :type E_Stats%20Enum :default "NewEnumerator0") (Value :type Float%20%28double-precision%29))
  (if (!= Value 0.0)
    (bind _output_get (LocalVariables|SetL_Value (+ (CallFunction|GetCurrentStatValue Stat) Value)))
    (bind _output_get_2 (LocalVariables|SetL_Value (Math|Float|Clamp(Float) _output_get 0.0 (CallFunction|GetMaxStatValue Stat))))
    (CallFunction|SetCurrentStatValue Stat _output_get_2)))

(fn GetBaseStats
  (params (Key :type E_Stats%20Enum%20%28by%20ref%29 :default "NewEnumerator0"))
  (return (.basevalue (.Value (Utilities|Map|Find (Variables|BaseStats|GetBaseStats) Key)))))

(fn GetMaxStatValue
  (params (Key :type E_Stats%20Enum%20%28by%20ref%29 :default "NewEnumerator0"))
  (return (.maxvalue (.Value (Utilities|Map|Find (Variables|BaseStats|GetBaseStats) Key)))))

(fn SetBaseStatValue
  (params (Stat :type E_Stats%20Enum :default "NewEnumerator0") (Value :type Float%20%28double-precision%29))
  (bind _structout (Utilities|Struct|SetmembersinF_BaseStats (.Value (Utilities|Map|Find (Variables|BaseStats|GetBaseStats) Stat)) Value))
  (Utilities|Map|Add (Variables|BaseStats|GetBaseStats) Stat _structout))

(fn SetMaxStatValue
  (params (Stat :type E_Stats%20Enum :default "NewEnumerator0") (Value :type Float%20%28double-precision%29))
  (bind _structout (Utilities|Struct|SetmembersinF_BaseStats (.Value (Utilities|Map|Find (Variables|BaseStats|GetBaseStats) Stat)) Value))
  (Utilities|Map|Add (Variables|BaseStats|GetBaseStats) Stat _structout))

(fn TakeDamage
  (params (InDamage :type Float%20%28double-precision%29))
  (CallFunction|ModifyCurrentStatValue "NewEnumerator1" (* InDamage -1.0))
  (if (<= (CallFunction|GetCurrentStatValue "NewEnumerator1") 0.0)
    (Default|Die (Actor|GetComponentbyClass (Components|GetOwner) "/Game/ParkourData/Blueprints/Components/ParkourComponent.ParkourComponent_C"))
    (return true)
    (else
      (return false))))