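; BP_PullPickUps is a helper actor that pulls nearby pickups toward its instigator, presumably the player.
; Shortly after BeginPlay it sets its Sphere component radius from the PullArea variable.
; Every Tick it queries the sphere for overlapping BP_PickUpActor actors and sends each a PullToPlayer message with the instigator's current location, leaving the movement to the pickup.
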(event EventTick
  (params (DeltaSeconds :type Float%20%28single-precision%29))
  (for _array_element (Collision|GetOverlappingActors (Variables|Default|GetSphere) "/Game/ParkourData/Blueprints/Actors/BP_PickUpActor.BP_PickUpActor_C" :!class /Script/Engine.PrimitiveComponent)
    (Class|InteractableBPI|PulltoPlayer(Message) _array_element (Transformation|GetActorLocation (Game|GetInstigator)))))

(event EventBeginPlay
  (Utilities|FlowControl|Delay 0.1)
  (Components|Sphere|SetSphereRadius (Variables|Default|GetSphere) (Variables|Default|GetPullArea) true))

(fn ConstructionScript)